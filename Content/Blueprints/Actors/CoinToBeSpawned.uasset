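; CoinToBeSpawned is a currency pickup coin that the player collects by touching it.
; On overlap with Player_BP, it passes its CoinValue to WaveGameMode_BP's UpdatePlayerCurrency and destroys itself, with debug prints on overlaps.
; Tick sets the Coin component's absolute world pitch from DeltaSeconds alone, so the rotation does not accumulate into a continuous spin.
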(event EventBeginPlay)

(event Collision|EventActorBeginOverlap
  (params (OtherActor :type Actor%20Object%20Reference))
  (Utilities|Casting|CastToPlayer_BP OtherActor
    (:then
      (Development|PrintString "Hello")
      (bind _aswave_game_mode_bp (Utilities|Casting|CastToWaveGameMode_BP (Game|GetGameMode)))
      (Class|WaveGameMode|UpdatePlayerCurrency _aswave_game_mode_bp (Variables|Default|GetCoinValue))
      (Actor|DestroyActor))
    (:CastFailed
      (Development|PrintString "Bye"))))

(event EventTick
  (params (DeltaSeconds :type Float%20%28single-precision%29))
  (Transformation|SetWorldRotation (Variables|Default|GetCoin) (Math|Rotator|MakeRotator 0.0 (* DeltaSeconds 2e+01) 0.0) false false))

(fn ConstructionScript)