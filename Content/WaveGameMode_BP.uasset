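; WaveGameMode_BP is a game mode for wave-based enemy spawning.
; On BeginPlay it gathers every EnemySpawner actor in the level into the EnemySpawners array.
; The SpawnNewEnemy event forwards an enemy type and route to the first spawner in that array only.
; BeginWave is an empty stub, and a disconnected debug print of the enemy total never runs.
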(event EventBeginPlay
  (Utilities|FlowControl|Sequence
    (:then_0
      (Utilities|Array|Clear (Variables|Default|GetEnemySpawners))
      (bind _outactors (Actor|GetAllActorsOfClass "/Game/AI/EnemySpawner.EnemySpawner_C"))
      (for _array_element _outactors
        (Utilities|Array|Add (Variables|Default|GetEnemySpawners) _array_element)))))

(event EventSpawnNewEnemy
  (params (EnemyToSpawn :type Pawn%20Class%20Reference) (RouteForEnemyToFollow :type Integer))
  (Default|SpawnEnemy (Utilities|Array|Get(acopy) (Variables|Default|GetEnemySpawners)) EnemyToSpawn RouteForEnemyToFollow))

(fn ConstructionScript)

(fn BeginWave)