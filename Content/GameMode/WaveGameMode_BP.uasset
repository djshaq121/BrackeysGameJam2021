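; Game mode for a wave-based game that handles enemy spawning and relays wave state to the HUD.
; On BeginPlay it caches all EnemySpawner actors, and SpawnNewEnemy asks the first one to spawn a given enemy type along a given route.
; Update events cast WaveSystemWidget to WaveSystem_Widget and push wave count, enemies left, lives, currency and the prepare-wave state.
; BeginWave is an empty function here.
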(event EventBeginPlay
  (Utilities|FlowControl|Sequence
    (:then_0
      (Utilities|Array|Clear (Variables|Default|GetEnemySpawners))
      (bind _outactors (Actor|GetAllActorsOfClass "/Game/AI/EnemySpawner.EnemySpawner_C"))
      (for _array_element _outactors
        (Utilities|Array|Add (Variables|Default|GetEnemySpawners) _array_element)))))

(event EventSpawnNewEnemy
  (params (EnemyToSpawn :type Pawn%20Class%20Reference) (RouteForEnemyToFollow :type Integer))
  (Default|SpawnEnemy (Utilities|Array|Get(acopy) (Variables|Default|GetEnemySpawners)) EnemyToSpawn RouteForEnemyToFollow))

(event EventUpdateWidgetonWaveStart
  (bind _aswave_system_widget (Utilities|Casting|CastToWaveSystem_Widget (Variables|Default|GetWaveSystemWidget)))
  (Default|SetPrepareWave _aswave_system_widget false))

(event EventUpdateWaveWidget
  (params (wave :type Integer) (totalWaves :type Integer))
  (bind _aswave_system_widget (Utilities|Casting|CastToWaveSystem_Widget (Variables|Default|GetWaveSystemWidget)))
  (Default|UpdateWave _aswave_system_widget wave totalWaves))

(event EventUpdateEnemiesLeftWidget
  (params (enemiesLeft :type Integer))
  (bind _aswave_system_widget (Utilities|Casting|CastToWaveSystem_Widget (Variables|Default|GetWaveSystemWidget)))
  (Default|UpdateEnemiesLeft _aswave_system_widget enemiesLeft))

(event EventUpdateChancesLeftWidget
  (params (Lives :type Integer))
  (bind _aswave_system_widget (Utilities|Casting|CastToWaveSystem_Widget (Variables|Default|GetWaveSystemWidget)))
  (Default|UpdateChances _aswave_system_widget Lives))

(event EventUpdateCurrencyWidget
  (params (currency :type Integer))
  (bind _aswave_system_widget (Utilities|Casting|CastToWaveSystem_Widget (Variables|Default|GetWaveSystemWidget)))
  (Default|UpdateCurrency _aswave_system_widget currency))

(event EventUpdateonPrepareforWave
  (bind _aswave_system_widget (Utilities|Casting|CastToWaveSystem_Widget (Variables|Default|GetWaveSystemWidget)))
  (Default|SetPrepareWave _aswave_system_widget true))

(fn ConstructionScript)

(fn BeginWave)